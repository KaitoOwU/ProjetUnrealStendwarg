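; Player controller for the main character that handles movement, camera look and changing glasses filters through Enhanced Input.
; BeginPlay adds the input mapping context and caches the BP_MainCharacter found in the level with GetActorOfClass.
; Move input drives that character along its forward and right vectors, and camera input adds controller yaw and pitch.
; Glasses input fires an event dispatcher with the current color, leaving the filter change to its listeners.
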(event Input|EnhancedActionEvents|EnhancedInputActionIA_Move
  (params (ActionValue :type Vector%202D%20Structure) (ElapsedSeconds :type Float%20%28double-precision%29) (TriggeredSeconds :type Float%20%28double-precision%29) (InputAction :type Input%20Action%20Object%20Reference :default "/Game/Project/Inputs/InputsActions/IA_Move.IA_Move"))
  (bind _maincharacter (Variables|Default|GetMainCharacter))
  ;[1 1 1] Character Movement
  (:Triggered
    (Pawn|Input|AddMovementInput _maincharacter (Transformation|GetActorForwardVector _maincharacter) (.x ActionValue) false)
    (Pawn|Input|AddMovementInput _maincharacter (Transformation|GetActorRightVector _maincharacter) (.y ActionValue) false)))

(event Input|EnhancedActionEvents|EnhancedInputActionIA_CameraMovement
  (params (ActionValue :type Vector%202D%20Structure) (ElapsedSeconds :type Float%20%28double-precision%29) (TriggeredSeconds :type Float%20%28double-precision%29) (InputAction :type Input%20Action%20Object%20Reference :default "/Game/Project/Inputs/InputsActions/IA_CameraMovement.IA_CameraMovement"))
  ;[1 1 1] Camera Movement
  (:Triggered
    (Class|PlayerController|AddYawInput (.x ActionValue))
    (Class|PlayerController|AddPitchInput (.y ActionValue))))

(event Input|EnhancedActionEvents|EnhancedInputActionIA_ChangeGlasses
  (params (ActionValue :type Boolean) (ElapsedSeconds :type Float%20%28double-precision%29) (TriggeredSeconds :type Float%20%28double-precision%29) (InputAction :type Input%20Action%20Object%20Reference :default "/Game/Project/Inputs/InputsActions/IA_ChangeGlasses.IA_ChangeGlasses"))
  ;[1 1 1] Change Glasses Filters
  (:Started
    (Default|CallEDChangeGlasses (Variables|Default|GetCurrentColor))))

(event EventBeginPlay
  (bind _returnvalue (PlayerController|LocalPlayerSubsystems|GetEnhancedInputLocalPlayerSubsystem))
  ;[1 1 1] Mapping Context
  (Utilities|IsValid _returnvalue
    (:Is%20Valid
      (Input|AddMappingContext _returnvalue "/Game/Project/Inputs/IMC_InputMappingContext.IMC_InputMappingContext" 0 "(bIgnoreAllPressedKeysUntilRelease=True,bForceImmediately=False)")
      (bind _returnvalue_2 (Actor|GetActorOfClass "/Game/Project/GameObjects/BP/BP_MainCharacter.BP_MainCharacter_C"))
      (Variables|Default|SetMainCharacter _returnvalue_2))))

(fn ConstructionScript)