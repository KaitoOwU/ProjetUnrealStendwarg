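; Colored block that shows or hides as the player changes the active glasses color filter.
; On BeginPlay it binds to the glasses-change dispatcher on PC_MainCharacter, which drives SwitchVisibility from the controller's current color.
; The mesh hides when its color matches the filter and shows otherwise, changing visibility only, not collision.
; A block colored None prints a setup warning whenever a color filter is active.
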(event Custom|SwitchBlockVisibility
  (params (CurrentColor :type E_Colors%20Enum%20%28by%20ref%29 :default "NewEnumerator0"))
  (CallFunction|SwitchVisibility (stale EventBeginPlay _aspc_main_character)))

(event EventBeginPlay
  (bind _aspc_main_character (Utilities|Casting|CastToPC_MainCharacter (Game|GetPlayerController 0)))
  (EventDispatchers|BindEventtoEDChangeGlasses _aspc_main_character (delegate Custom|SwitchBlockVisibility)))

(fn ConstructionScript)

(fn SwitchVisibility
  (params (currentColor :type PC%20Main%20Character%20Object%20Reference%20%28by%20ref%29))
  (bind _blockmesh (Variables|Default|GetBlockMesh))
  (bind _blockcolor (Variables|Default|GetBlockColor))
  ;[1 1 1] Switch Visibility based on current active filter, and block color
  (switch Utilities|FlowControl|Switch|SwitchonE_Colors (Variables|/Game/Project/GameObjects/Game/PC_MainCharacter.PC_MainCharacter_C|GetCurrentColor currentColor)
    (:NewEnumerator0
      (switch Utilities|FlowControl|Switch|SwitchonE_Colors _blockcolor
        (:NewEnumerator0
          (Rendering|SetVisibility _blockmesh false false :!label _label))
        (:NewEnumerator1
          (Rendering|SetVisibility _blockmesh true false :!label _label_2))
        (:NewEnumerator2
          (Development|PrintString "A block cannot be of color \"None\". If you don't want this block to be affected by the filter change, you can just remove \"BP_BlockActor\" from it." true true "(R=0.000000,G=0.660000,B=1.000000,A=1.000000)" 1e+01 :!pinned true :!label _label_3) ; Debug
        )))
    (:NewEnumerator1
      (switch Utilities|FlowControl|Switch|SwitchonE_Colors _blockcolor
        (:NewEnumerator0
          (goto _label_2))
        (:NewEnumerator1
          (goto _label))
        (:NewEnumerator2
          (goto _label_3))))
    (:NewEnumerator2
      (goto _label_2))))