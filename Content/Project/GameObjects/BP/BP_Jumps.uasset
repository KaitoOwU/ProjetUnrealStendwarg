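; Handles the main character's jump and charged pickaxe launch from the IA_ChargeJump input.
; Holding accumulates Charge, with sound cues near each fifth of MaxCharge.
; On release, a sphere trace at the feet gates a normal jump, or a launch if charge exceeds the threshold and level data enables the pickaxe.
; Launches follow the controller's forward vector with upward bias, scaled by charge; separate grounded-state updates notify BP_WallMoves.
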(event Input|EnhancedActionEvents|EnhancedInputActionIA_ChargeJump
  (params (ActionValue :type Boolean) (ElapsedSeconds :type Float%20%28double-precision%29) (TriggeredSeconds :type Float%20%28double-precision%29) (InputAction :type Input%20Action%20Object%20Reference :default "/Game/Project/Inputs/InputsActions/IA_ChargeJump.IA_ChargeJump"))
  (:Triggered
    (CallFunction|AddChargePower))
  (:Started
    (Variables|Default|SetCharge 0.0))
  (:Completed
    (bind _returnvalue (CallFunction|Groundcheck))
    ;[1 0.1631 0.1962] Check if the player can jump
    (if _returnvalue
      ;[1 1 1] Check whether to do a simple jump or launch the player
      (if (and (> (Variables|Default|GetCharge) (Variables|Default|GetPowerThreshold)) (Variables|Default|GetIsPickaxeEquipped))
        (CallFunction|PickaxeLaunch (Variables|Default|GetCharge))
        (else
          (CallFunction|SetJump)))
      (Variables|Default|SetCharge 0.0)
      (else
        (Development|PrintString "Can't Jump / Launch")
        (Variables|Default|SetCharge 0.0)))))

(event EventBeginPlay
  ;[1 1 1] Sets the player controller as a variable
  (bind _aspc_main_character (Utilities|Casting|CastToPC_MainCharacter (Game|GetPlayerController 0)))
  (Variables|Default|SetAs%20PC%20Main%20Character _aspc_main_character)
  ;[1 1 1] Sets the character as a variable
  (bind _asbp_main_character (Utilities|Casting|CastToBP_MainCharacter (Game|GetPlayerCharacter 0)))
  (Variables|Default|SetAs%20BP%20Main%20Character _asbp_main_character)
  ;[1 1 1] Check if pickaxe active
  (bind _asgi_stendvarg (Utilities|Casting|CastToGI_Stendvarg (Game|GetGameInstance)))
  (Variables|Default|SetIsPickaxeEquipped (.PickaxeActive (Utilities|Struct|BreakS_LevelData (Variables|/Game/Project/GameObjects/Game/GI_Stendvarg.GI_Stendvarg_C|GetCurrentLevelData _asgi_stendvarg)))))

(fn AddChargePower
  (bind _maxcharge (Variables|Default|GetMaxCharge))
  (bind _returnvalue (/ _maxcharge 5.0))
  (bind _output_get (Variables|Default|SetCharge (+ (Variables|Default|GetCharge) (Utilities|Time|GetWorldDeltaSeconds))))
  (if (Math|Float|NearlyEqual(Float) _output_get _returnvalue 0.0001)
    (Audio|PlaySound2D "/Game/Project/SoundDesign/SoundEffetcs/Pickaxe/charge_pickaxe_lvl_1__1_.charge_pickaxe_lvl_1__1_" 1.1 0.7 0.0 0 0)
    (Development|PrintString "Hello" :!label _label)
    (elif (Math|Float|NearlyEqual(Float) _output_get (* _returnvalue 2.0) 0.01)
      (Audio|PlaySound2D "/Game/Project/SoundDesign/SoundEffetcs/Pickaxe/charge_pickaxe_lvl_2__1_.charge_pickaxe_lvl_2__1_" 1.1 0.7 0.0 0 0)
      (goto _label)
      (elif (Math|Float|NearlyEqual(Float) _output_get (* _returnvalue 3.0) 0.01)
        (Audio|PlaySound2D "/Game/Project/SoundDesign/SoundEffetcs/Pickaxe/charge_pickaxe_lvl_3__1_.charge_pickaxe_lvl_3__1_" 1.1 0.7 0.0 0 0)
        (goto _label)
        (elif (Math|Float|NearlyEqual(Float) _output_get (* _returnvalue 4.0) 0.01)
          (Audio|PlaySound2D "/Game/Project/SoundDesign/SoundEffetcs/Pickaxe/charge_pickaxe_lvl_4__1_.charge_pickaxe_lvl_4__1_" 1.1 0.7 0.0 0 0)
          (goto _label)
          (elif (Math|Float|NearlyEqual(Float) _output_get _maxcharge 0.01)
            (Audio|PlaySound2D "/Game/Project/SoundDesign/SoundEffetcs/Pickaxe/charge_pickaxe_lvl_5__1_.charge_pickaxe_lvl_5__1_" 1.1 0.7 0.0 0 0)
            (goto _label)))))))

(fn SetJump
  (Character|Jump (Game|GetPlayerCharacter 0))
  (Development|PrintString "Jumped"))

(fn PickaxeLaunch
  (params (LaunchingPower :type Float%20%28double-precision%29))
  (bind _launchdirection (CallFunction|SetLaunch (Variables|Default|GetAs%20PC%20Main%20Character) (Math|Float|Clamp(Float) LaunchingPower 0.0 (Variables|Default|GetMaxCharge))))
  (Character|LaunchCharacter (Game|GetPlayerCharacter 0) (Math|Vector|MakeVector (.x _launchdirection) (.y _launchdirection) (.z _launchdirection)) false false)
  ;[1 1 1] Sound
  (Utilities|FlowControl|MultiGate true false -1
    (:Out%200
      (Audio|SpawnSound2D "/Game/Project/SoundDesign/SoundEffetcs/Pickaxe/coup_pioche_1.coup_pioche_1" 1.0 1.0 0.0 0))
    (:Out%201
      (Audio|SpawnSound2D "/Game/Project/SoundDesign/SoundEffetcs/Pickaxe/Coup_pioche_2.Coup_pioche_2" 1.0 1.0 0.0 0))
    (:Out%202
      (Audio|SpawnSound2D "/Game/Project/SoundDesign/SoundEffetcs/Pickaxe/Coup_pioche_3.Coup_pioche_3" 1.0 1.0 0.0 0))))

(fn SetLaunch
  (params (self2 :type Actor%20Object%20Reference) (LaunchCharge :type Float%20%28double-precision%29))
  (bind _returnvalue (Transformation|GetActorForwardVector self2))
  (bind _maxcharge (Variables|Default|GetMaxCharge))
  (bind _launchpower (Variables|Default|GetLaunchPower))
  (bind _returnvalue_2 (/ LaunchCharge _maxcharge))
  (bind _returnvalue_3 (* _launchpower _returnvalue_2))
  (Development|PrintString (Utilities|String|ToString(Float) _returnvalue_3) true true "(R=0.491000,G=1.000000,B=1.000000,A=1.000000)" 1.0)
  (return (Math|Vector|ClampVectorSize (* (Math|Vector|MakeVector (.x _returnvalue) (.y _returnvalue) (Math|Float|Clamp(Float) (.z _returnvalue) 1.4 2.0)) _returnvalue_3) 0.0 (Variables|Default|GetLaunchPower)) _returnvalue_3))

(fn UpdateGroundedBool
  (params (Grounded :type Boolean))
  ;[1 1 1] Toggles the bool
  (bind _output_get (Variables|Default|SetIsGrounded Grounded))
  (Default|JumpUpdate (Actor|GetComponentbyClass (Variables|Default|GetAs%20BP%20Main%20Character) "/Game/Project/GameObjects/BP/BP_WallMoves.BP_WallMoves_C"))
  ;[1 1 1] Debug
  (Development|PrintString (Utilities|String|ToString(Boolean) _output_get) true true "(R=1.000000,G=1.000000,B=1.000000,A=1.000000)" 1.0)
  (return _output_get))

(fn Groundcheck
  (bind _as_bp_main_character (Variables|Default|GetAs%20BP%20Main%20Character))
  (bind _returnvalue (Transformation|GetActorLocation _as_bp_main_character))
  (bind _returnvalue_2 (- (.z _returnvalue) 88.0))
  (bind _returnvalue_3 (Math|Vector|MakeVector (.x _returnvalue) (.y _returnvalue) _returnvalue_2))
  (bind _returnvalue_4 (Collision|SphereTraceByChannel _returnvalue_3 _returnvalue_3 25.0 "TraceTypeQuery4" false 0 "ForDuration" true "(R=1.000000,G=0.000000,B=0.000000,A=1.000000)" "(R=0.000000,G=1.000000,B=0.000000,A=1.000000)" 2.0))
  (return _returnvalue_4))