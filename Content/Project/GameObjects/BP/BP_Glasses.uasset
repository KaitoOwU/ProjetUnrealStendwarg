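; BP_Glasses is the glasses object that cycles the player's current color.
; On BeginPlay it casts the first player controller to PC_MainCharacter and binds to its change-glasses event dispatcher.
; Each dispatch advances a looping, sequential MultiGate that writes one of three enum values into the controller's CurrentColorVar.
; The SwitchColour function is a stub holding only an unconnected MultiGate.
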(event Custom|ED_ChangeGlasses_Event
  ;[1 1 1] Switch Color
  (Utilities|FlowControl|MultiGate false true -1
    (:Out%200
      (|SetBy-RefVar (Variables|/Game/Project/GameObjects/Game/PC_MainCharacter.PC_MainCharacter_C|GetCurrentColorVar (stale EventBeginPlay _aspc_main_character)) "NewEnumerator0"))
    (:Out%201
      (|SetBy-RefVar (Variables|/Game/Project/GameObjects/Game/PC_MainCharacter.PC_MainCharacter_C|GetCurrentColorVar (stale EventBeginPlay _aspc_main_character)) "NewEnumerator1"))
    (:Out%202
      (|SetBy-RefVar (Variables|/Game/Project/GameObjects/Game/PC_MainCharacter.PC_MainCharacter_C|GetCurrentColorVar (stale EventBeginPlay _aspc_main_character)) "NewEnumerator2"))))

(event EventBeginPlay
  (bind _aspc_main_character (Utilities|Casting|CastToPC_MainCharacter (Game|GetPlayerController 0)))
  (EventDispatchers|BindEventtoEDChangeGlasses _aspc_main_character (delegate Custom|ED_ChangeGlasses_Event)))

(fn SwitchColour
  (Utilities|FlowControl|MultiGate false true 1))