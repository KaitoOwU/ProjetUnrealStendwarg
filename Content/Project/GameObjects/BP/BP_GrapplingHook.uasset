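; Grappling hook component for BP_MainCharacter that pulls the player toward hook actors in the level.
; StartGrappling line-traces for an actor implementing I_IsHook, switches movement to Flying, stores the hook's location and calls the wall-move component's CheckWREnd.
; Tick applies force toward that point until within drop range, then StopGrappling restores Walking and halts movement, or launches the character when keeping inertia.
; IsAimingHook reports any trace hit, without checking the interface.
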(event EventTick
  (params (DeltaSeconds :type Float%20%28single-precision%29))
  (if (Variables|Default|GetIsGrappling)
    (Physics|AddForce (Variables|Default|GetCharacterMovement) (* (Math|Vector|Normalize (Math|Vector|GetUnitDirection(Vector) (Transformation|GetActorLocation (Variables|Default|GetMainCharacter)) (Variables|Default|GetGrappleHookLocation))) (Variables|Default|GetGrapplingHookSpeed)))
    (if (<= (Math|Vector|Distance(Vector) (Transformation|GetActorLocation (Variables|Default|GetMainCharacter)) (Variables|Default|GetGrappleHookLocation)) (Variables|Default|GetHookRangeBeforeDrop))
      (CallFunction|StopGrappling false))))

(event EventBeginPlay
  (bind _asbp_main_character (Utilities|Casting|CastToBP_MainCharacter (Components|GetOwner)))
  (bind _output_get (Variables|Default|SetMainCharacter _asbp_main_character))
  (Variables|Default|SetCharacterMovement (Variables|/Script/Engine.Character|GetCharacterMovement _output_get)))

(fn StartGrappling
  ;[1 1 1] Check if Grappling is Possible then Line Trace
  (if (not (Variables|Default|GetIsGrappling))
    (bind _asbp_main_character (Utilities|Casting|CastToBP_MainCharacter (Components|GetOwner)))
    (bind (_outhit _returnvalue) (Collision|LineTraceByChannel (.Start (Utilities|GetLineTraceStartandEnd _asbp_main_character)) (.End (Utilities|GetLineTraceStartandEnd _asbp_main_character)) "TraceTypeQuery3" false 0 "ForDuration"))
    (if (and _returnvalue (Utilities|DoesObjectImplementInterface (.HitActor (Collision|BreakHitResult _outhit)) "/Game/Project/GameObjects/BP/I_IsHook.I_IsHook_C"))
      (Variables|Default|SetIsGrappling true)
      (Pawn|Components|CharacterMovement|SetMovementMode (Variables|Default|GetCharacterMovement) "MOVE_Flying" 0)
      (Variables|Default|SetGrappleHookLocation (Transformation|GetActorLocation (.HitActor (Collision|BreakHitResult _outhit))))
      (Default|CheckWREnd (Variables|/Game/Project/GameObjects/BP/LevelDesign/BP_MainCharacter.BP_MainCharacter_C|GetBP_WallMoves (Variables|Default|GetMainCharacter))))))

(fn StopGrappling
  (params (KeepInertia :type Boolean))
  (bind _maincharacter (Variables|Default|GetMainCharacter))
  (bind _charactermovement (Variables|Default|GetCharacterMovement))
  (if (Variables|Default|GetIsGrappling)
    (Pawn|Components|CharacterMovement|SetMovementMode _charactermovement "MOVE_Walking" 0)
    (Variables|Default|SetIsGrappling false)
    (if KeepInertia
      (Character|LaunchCharacter _maincharacter (+ (* (Math|Vector|Normalize (Math|Vector|GetUnitDirection(Vector) (Transformation|GetActorLocation _maincharacter) (Variables|Default|GetGrappleHookLocation))) 0.5) (Math|Vector|MakeVector 0.0 0.0 (Variables|Default|GetInertia))) false false)
      (else
        (Components|Movement|StopMovementImmediately _charactermovement)))))

(fn IsAimingHook
  (bind _maincharacter (Variables|Default|GetMainCharacter))
  (bind (_start _end) (Utilities|GetLineTraceStartandEnd _maincharacter))
  (bind _returnvalue (Collision|LineTraceByChannel _start _end "TraceTypeQuery3" false 0 "None"))
  (return _returnvalue))