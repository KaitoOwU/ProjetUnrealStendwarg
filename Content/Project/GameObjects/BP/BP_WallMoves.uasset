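; Blueprint that gives BP_MainCharacter wall running and wall jumping.
; Left/right wall-contact events and ground checks start or end runs through ON/OFF dispatchers, which scale gravity and air control.
; While running, Tick line-traces sideways for the wall normal, pushing the player into the wall and upward, and ends the run on a miss.
; Releasing charge-jump launches off the wall; sliding sound and sparks start only on right-side runs.
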(event Custom|LWRON
  ;[1 0 0.05758] When the player starts/stops touching a wall
  (Variables|Default|SetLeftWR true)
  (CallFunction|UpdateWallRun))

(event Custom|RWRON
  ;[1 0 0.05758] When the player starts/stops touching a wall
  (Variables|Default|SetRightWR true)
  (CallFunction|UpdateWallRun))

(event Custom|EDCalled3
  (params (IsWRing :type Boolean) (WasWRRight :type Boolean) (IsLaunching :type Boolean))
  ;[1 1 1] Begin Play
  (bind _output_get (Variables|Default|SetIsWRing IsWRing))
  (CallFunction|UpdatePlayerMovements _output_get)
  (if IsLaunching
    (CallFunction|JumpOffWall))
  (bind _wallrunsound (Variables|Default|GetWallRunSound)
    (:then
      (Audio|Components|Audio|Stop _wallrunsound))
    (:else
      _))
  (Components|Activation|SetActive (Variables|/Game/Project/GameObjects/BP/LevelDesign/BP_MainCharacter.BP_MainCharacter_C|GetSparks (Variables|Default|GetAs%20BP%20Main%20Character)) false false))

(event Custom|UpdateWallRun
  ;[0 0.3764 0.1313] Called on each groundcheck or wallcheck
  (if (not (Variables|Default|GetIsWRing))
    (bind _returnvalue (Default|Groundcheck (Variables|/Game/Project/GameObjects/BP/LevelDesign/BP_MainCharacter.BP_MainCharacter_C|GetBP_Jumps (Variables|Default|GetAs%20BP%20Main%20Character))))
    (if (and (not _returnvalue) (Variables|Default|GetCanWallRun))
      (CallFunction|StartWallrunning)
      (else
        (Audio|Components|Audio|Stop (Variables|Default|GetWallRunSound))
        (Components|Activation|SetActive (Variables|/Game/Project/GameObjects/BP/LevelDesign/BP_MainCharacter.BP_MainCharacter_C|GetSparks (Variables|Default|GetAs%20BP%20Main%20Character)) false false)))))

(event Custom|LWROFF
  ;[1 0 0.05758] When the player starts/stops touching a wall
  (Variables|Default|SetLeftWR false)
  (CallFunction|UpdateWallRun))

(event Custom|RWROFF
  ;[1 0 0.05758] When the player starts/stops touching a wall
  (Variables|Default|SetRightWR false)
  (CallFunction|UpdateWallRun))

(event Custom|JumpUpdate
  ;[0 0.4798 1] GroundCheck
  (bind _returnvalue (Default|Groundcheck (Variables|/Game/Project/GameObjects/BP/LevelDesign/BP_MainCharacter.BP_MainCharacter_C|GetBP_Jumps (Variables|Default|GetAs%20BP%20Main%20Character))))
  (if _returnvalue
    (Variables|Default|SetCanWallRun true)
    (CallFunction|CheckWREnd)
    (else
      (CallFunction|UpdateWallRun))))

(event Custom|EDCalled2
  (params (IsWRing :type Boolean) (IsWRingRight :type Boolean))
  ;[1 1 1] Begin Play
  (CallFunction|UpdatePlayerMovements IsWRing))

(event Input|EnhancedActionEvents|EnhancedInputActionIA_ChargeJump
  (params (ActionValue :type Boolean) (ElapsedSeconds :type Float%20%28double-precision%29) (TriggeredSeconds :type Float%20%28double-precision%29) (InputAction :type Input%20Action%20Object%20Reference :default "/Game/Project/Inputs/InputsActions/IA_ChargeJump.IA_ChargeJump"))
  ;[1 0.9776 0.007091] WallJump
  (:Completed
    (if (Variables|Default|GetIsWRing)
      (Default|CallEDWallrunningOFF false (Variables|Default|GetWRingRight) true)
      (bind _wallrunsound (Variables|Default|GetWallRunSound)
        (:then
          (Audio|Components|Audio|Stop _wallrunsound))
        (:else
          _))
      (Components|Activation|SetActive (Variables|/Game/Project/GameObjects/BP/LevelDesign/BP_MainCharacter.BP_MainCharacter_C|GetSparks (Variables|Default|GetAs%20BP%20Main%20Character)) false false))))

(event EventBeginPlay
  ;[1 1 1] Begin Play
  (bind _asbp_main_character (Utilities|Casting|CastToBP_MainCharacter (Game|GetPlayerCharacter 0)))
  (Variables|Default|SetAs%20BP%20Main%20Character _asbp_main_character)
  (EventDispatchers|BindEventtoEDWallrunningON (delegate Custom|EDCalled2))
  (EventDispatchers|BindEventtoEDWallrunningOFF (delegate Custom|EDCalled3))
  (CallFunction|SetInitialMovementsValues))

(event EventTick
  (params (DeltaSeconds :type Float%20%28single-precision%29))
  ;[0.3673 0.3673 0.3673] WALLRUNNING
  (if (Variables|Default|GetIsWRing)
    (bind (_start _end) (CallFunction|GetWRVector))
    (bind (_charactermovement _impactpoint _normal_vector) (CallFunction|GetSurfaceNormal _start _end))
    (Physics|AddForce _charactermovement (+ (* _normal_vector -2.5e+03) "0.000000,0.000000,800.000000"))))

(fn StartWallrunning
  (if (and (Variables|Default|GetLeftWR) (Variables|Default|GetRightWR))
    (Development|PrintString "Facing the wall rn" true true "(R=1.000000,G=0.065008,B=0.000000,A=1.000000)" 1.0)
    (Default|CallEDWallrunningOFF false (Variables|Default|GetWRingRight) false)
    (Audio|Components|Audio|Stop (Variables|Default|GetWallRunSound))
    (Components|Activation|SetActive (Variables|/Game/Project/GameObjects/BP/LevelDesign/BP_MainCharacter.BP_MainCharacter_C|GetSparks (Variables|Default|GetAs%20BP%20Main%20Character)) false false)
    (else
      ;[0.9667 1 0] Wallrunning Left
      (if (Variables|Default|GetLeftWR)
        (Development|PrintString "LEFT WALLRUNNING RN" true true "(R=0.000000,G=1.000000,B=0.927135,A=1.000000)" 1.0)
        (bind _output_get (Variables|Default|SetWRingRight false))
        (bind _output_get_2 (Variables|Default|SetIsWRing true))
        (Default|CallEDWallrunningON _output_get_2 _output_get)
        (else
          ;[0.177 0.3553 1] Wallrunning Right
          (if (Variables|Default|GetRightWR)
            (Development|PrintString "RIGHT WALLRUNNING RN" true true "(R=0.000000,G=1.000000,B=0.927135,A=1.000000)" 1.0)
            (bind _output_get_3 (Variables|Default|SetWRingRight true))
            (bind _output_get_4 (Variables|Default|SetIsWRing true))
            (Default|CallEDWallrunningON _output_get_4 _output_get_3)
            ;[1 1 1] Sound
            (bind _returnvalue (Audio|SpawnSound2D "/Game/Project/SoundDesign/SoundEffetcs/Slide/Soundeffect_Sliding.Soundeffect_Sliding" 1.5 1.0 0.0 0))
            (Variables|Default|SetWallRunSound _returnvalue)
            (Components|Activation|SetActive (Variables|/Game/Project/GameObjects/BP/LevelDesign/BP_MainCharacter.BP_MainCharacter_C|GetSparks (Variables|Default|GetAs%20BP%20Main%20Character)) true false)))))))

(fn GetWRVector
  (bind _as_bp_main_character (Variables|Default|GetAs%20BP%20Main%20Character))
  (bind _returnvalue (Transformation|GetActorLocation _as_bp_main_character))
  (bind _capsulecomponent (Variables|/Script/Engine.Character|GetCapsuleComponent _as_bp_main_character))
  (if (Variables|Default|GetWRingRight)
    (return _returnvalue (+ _returnvalue (* (Math|Vector|GetRightVector _capsulecomponent) 1e+02)))
    (else
      (return _returnvalue (+ _returnvalue (* (Math|Vector|GetRightVector _capsulecomponent) -1e+02))))))

(fn GetSurfaceNormal
  (params (Start :type Vector) (End :type Vector))
  (bind _outhit (Collision|LineTraceByChannel Start End "TraceTypeQuery1" false 0 "ForDuration" true "(R=1.000000,G=1.000000,B=1.000000,A=1.000000)" "(R=1.000000,G=0.919292,B=0.000000,A=1.000000)" 0.5))
  (if (.bBlockingHit (Collision|BreakHitResult _outhit))
    (return (Variables|/Script/Engine.Character|GetCharacterMovement (Variables|Default|GetAs%20BP%20Main%20Character)) (.ImpactPoint (Collision|BreakHitResult _outhit)) (- (+ (.ImpactPoint (Collision|BreakHitResult _outhit)) (* (.ImpactNormal (Collision|BreakHitResult _outhit)) 2e+02)) (.ImpactPoint (Collision|BreakHitResult _outhit))))
    (else
      (Default|CallEDWallrunningOFF false (Variables|Default|GetWRingRight) false))))

(fn UpdatePlayerMovements
  (params (IsWRing :type Boolean))
  (bind _as_bp_main_character (Variables|Default|GetAs%20BP%20Main%20Character))
  (bind _charactermovement (Variables|/Script/Engine.Character|GetCharacterMovement _as_bp_main_character))
  (if IsWRing
    (Variables|/Script/Engine.CharacterMovementComponent|SetGravityScale _charactermovement (/ (Variables|Default|GetGravity%20Scale) 5.0))
    (Variables|/Script/Engine.CharacterMovementComponent|SetAirControl _charactermovement (/ (Variables|Default|GetAir%20Control) 6.0))
    (CallFunction|CorrectZVelocity)
    (else
      (Variables|/Script/Engine.CharacterMovementComponent|SetGravityScale _charactermovement (Variables|Default|GetGravity%20Scale))
      (Variables|/Script/Engine.CharacterMovementComponent|SetAirControl _charactermovement (Variables|Default|GetAir%20Control)))))

(fn JumpOffWall
  (bind _wallrunsound (Variables|Default|GetWallRunSound)
    (:then
      (Audio|Components|Audio|Stop _wallrunsound))
    (:else
      _))
  (bind (_start _end) (CallFunction|GetWRVector))
  (bind _normal_vector (CallFunction|GetSurfaceNormal _start _end))
  (Physics|AddImpulse (Variables|/Script/Engine.Character|GetCharacterMovement (Variables|Default|GetAs%20BP%20Main%20Character)) (+ (* _normal_vector 8.0) "0.000000,0.000000,800.000000") true)
  (CallFunction|CorrectZVelocity))

(fn SetInitialMovementsValues
  (bind _as_bp_main_character (Variables|Default|GetAs%20BP%20Main%20Character))
  (Variables|Default|SetGravity%20Scale (Variables|/Game/Project/GameObjects/BP/LevelDesign/BP_MainCharacter.BP_MainCharacter_C|GetGravityScaleSet _as_bp_main_character))
  (Variables|Default|SetAir%20Control (Variables|/Game/Project/GameObjects/BP/LevelDesign/BP_MainCharacter.BP_MainCharacter_C|GetAirControlSet _as_bp_main_character)))

(fn CheckWREnd
  (if (Variables|Default|GetIsWRing)
    (Default|CallEDWallrunningOFF false (Variables|Default|GetWRingRight) false)
    (Audio|Components|Audio|Stop (Variables|Default|GetWallRunSound))
    (Components|Activation|SetActive (Variables|/Game/Project/GameObjects/BP/LevelDesign/BP_MainCharacter.BP_MainCharacter_C|GetSparks (Variables|Default|GetAs%20BP%20Main%20Character)) false false)))

(fn CorrectZVelocity
  (bind _as_bp_main_character (Variables|Default|GetAs%20BP%20Main%20Character))
  (bind _charactermovement (Variables|/Script/Engine.Character|GetCharacterMovement _as_bp_main_character))
  (bind _velocity (Variables|/Script/Engine.MovementComponent|GetVelocity _charactermovement))
  (if (> (.z _velocity) 0.0)
    (Physics|AddImpulse _charactermovement (Math|Vector|MakeVector 0.0 0.0 (* (.z _velocity) -0.25)) true)
    (else
      (Physics|AddImpulse _charactermovement (Math|Vector|MakeVector 0.0 0.0 (* (.z _velocity) -1.1)) true))))