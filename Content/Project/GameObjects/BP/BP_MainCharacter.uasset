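; Player character Blueprint with grappling hook and wall-running support, applying gravity, walk speed and air control settings at BeginPlay.
; A hook collider is sized to the grapple range, and actor overlaps toggle nearby hooks active.
; GroundCheck overlaps fire a jump-update dispatcher, delayed briefly when contact ends.
; Left and right wall colliders test for runnable walls through an interface and update the wall-moves component.
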(event OnComponentBeginOverlap(GroundCheck)
  (params (OverlappedComponent :type Primitive%20Component%20Object%20Reference) (OtherActor :type Actor%20Object%20Reference) (OtherComp :type Primitive%20Component%20Object%20Reference) (OtherBodyIndex :type Integer) (bFromSweep :type Boolean) (SweepResult :type Hit%20Result%20Structure%20%28by%20ref%29))
  ;[1 1 1] Comment
  (Default|CallEDCanJumpUpdate))

(event OnComponentEndOverlap(GroundCheck)
  (params (OverlappedComponent :type Primitive%20Component%20Object%20Reference) (OtherActor :type Actor%20Object%20Reference) (OtherComp :type Primitive%20Component%20Object%20Reference) (OtherBodyIndex :type Integer))
  ;[1 1 1] Comment
  (Utilities|FlowControl|Delay 0.4)
  (Default|CallEDCanJumpUpdate))

(event OnComponentBeginOverlap(WallCheckL)
  (params (OverlappedComponent :type Primitive%20Component%20Object%20Reference) (OtherActor :type Actor%20Object%20Reference) (OtherComp :type Primitive%20Component%20Object%20Reference) (OtherBodyIndex :type Integer) (bFromSweep :type Boolean) (SweepResult :type Hit%20Result%20Structure%20%28by%20ref%29))
  ;[1 1 1] Comment
  (bind _isrunnable (CallFunction|IsWallrunnable OtherActor))
  (if _isrunnable
    (Default|UpdateWallRun (Variables|Default|GetBP_WallMoves) _isrunnable (stale OnComponentBeginOverlap(WallCheckR) _isrunnable))))

(event OnComponentBeginOverlap(WallCheckR)
  (params (OverlappedComponent :type Primitive%20Component%20Object%20Reference) (OtherActor :type Actor%20Object%20Reference) (OtherComp :type Primitive%20Component%20Object%20Reference) (OtherBodyIndex :type Integer) (bFromSweep :type Boolean) (SweepResult :type Hit%20Result%20Structure%20%28by%20ref%29))
  ;[1 1 1] Comment
  (bind _isrunnable (CallFunction|IsWallrunnable OtherActor))
  (if _isrunnable
    (Default|UpdateWallRun (Variables|Default|GetBP_WallMoves) (stale OnComponentBeginOverlap(WallCheckL) _isrunnable) _isrunnable)))

(event EventBeginPlay
  (bind _returnvalue (Game|GetPlayerCharacter 0))
  (bind _charactermovement (Variables|/Script/Engine.Character|GetCharacterMovement _returnvalue))
  (Components|Sphere|SetSphereRadius (Variables|Default|GetHookCollider) (Variables|/Game/Project/GameObjects/BP/BP_GrapplingHook.BP_GrapplingHook_C|GetGrapplingHookRange (Variables|Default|GetBP_GrapplingHook)) true)
  ;[1 1 1] Sets Character Values
  (Variables|/Script/Engine.CharacterMovementComponent|SetGravityScale _charactermovement (Variables|Default|GetGravityScaleSet))
  (Variables|/Script/Engine.CharacterMovementComponent|SetMaxWalkSpeed _charactermovement (Variables|Default|GetCharacterSpeed))
  (Variables|/Script/Engine.CharacterMovementComponent|SetAirControl _charactermovement (Variables|Default|GetAirControlSet)))

(event Collision|EventActorBeginOverlap
  (params (OtherActor :type Actor%20Object%20Reference))
  ;[1 1 1] Makes the hooks grappleable when near them
  (if (Utilities|DoesObjectImplementInterface OtherActor "/Game/Project/GameObjects/BP/I_IsHook.I_IsHook_C")
    (bind _asbp_hook (Utilities|Casting|CastToBP_Hook OtherActor))
    (Default|SetActive _asbp_hook true)))

(event Collision|EventActorEndOverlap
  (params (OtherActor :type Actor%20Object%20Reference))
  ;[1 1 1] Makes the hooks grappleable when near them
  (if (Utilities|DoesObjectImplementInterface OtherActor "/Game/Project/GameObjects/BP/I_IsHook.I_IsHook_C")
    (bind _asbp_hook (Utilities|Casting|CastToBP_Hook OtherActor))
    (Default|SetActive _asbp_hook false)))

(fn ConstructionScript)

(fn IsWallrunnable
  (params (InputActor :type Object%20Object%20Reference))
  (if (Utilities|DoesObjectImplementInterface InputActor "/Game/Project/GameObjects/BP/BI_Wallrun.BI_Wallrun_C")
    (bind _aswallrunable_wall (Utilities|Casting|CastToWallrunableWall InputActor))
    (return InputActor (Variables|/Game/Project/GameObjects/BP/WallrunableWall.WallrunableWall_C|GetIsRunnable _aswallrunable_wall))))