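; UI manager actor that runs the level's on-screen timer and reports the player's elapsed time.
; StartUIDisplay resets the time, creates a UW_UI widget, and uses a Timeline's update as a tick to accumulate delta seconds into it.
; StopUIDisplay removes the widget and stops the Timeline.
; Getter functions expose the elapsed time, formatted through ConvertTimeStamp as seconds and milliseconds.
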(event Custom|StartUIDisplay
  ;[1 1 1] Init and add time widget
  (Variables|Default|SetElapsedTime 0.0)
  (bind _returnvalue (UserInterface|CreateWidget "/Game/Project/UMG/UW_UI.UW_UI_C" (Variables|Default|GetPlayerController)))
  (UserInterface|Viewport|AddtoViewport _returnvalue 0)
  (Variables|Default|SetUiWidget _returnvalue)
  ;[1 1 1] Elapsed Time Update
  (Timeline|Timeline Play
    (:Update
      (bind _output_get (Variables|Default|SetElapsedTime (+ (Utilities|Time|GetWorldDeltaSeconds) (Variables|Default|GetElapsedTime))))
      (Variables|/Game/Project/UMG/UW_UI.UW_UI_C|SetTimeValue (Variables|Default|GetUiWidget) (.SS:MS (Utilities|ConvertTimeStamp _output_get))))))

(event Custom|StopUIDisplay
  ;[1 1 1] Remove Time Widget
  (Widget|RemovefromParent (Variables|Default|GetUiWidget))
  ;[1 1 1] Elapsed Time Update
  (Timeline|Timeline Stop
    (:Update
      (bind _output_get (Variables|Default|SetElapsedTime (+ (Utilities|Time|GetWorldDeltaSeconds) (Variables|Default|GetElapsedTime))))
      (Variables|/Game/Project/UMG/UW_UI.UW_UI_C|SetTimeValue (Variables|Default|GetUiWidget) (.SS:MS (Utilities|ConvertTimeStamp _output_get))))))

(event EventBeginPlay
  ;[1 1 1] Set PC
  (bind _aspc_main_character (Utilities|Casting|CastToPC_MainCharacter (Game|GetPlayerController 0)))
  (Variables|Default|SetPlayerController _aspc_main_character))

(fn ConstructionScript)

(fn GetLevelPerformance
  (bind _elapsedtime (Variables|Default|GetElapsedTime))
  (return (Utilities|Text|ToText(String) (.SS:MS (Utilities|ConvertTimeStamp _elapsedtime))) _elapsedtime))

(fn GetConvertedElapsedTime
  (return (Utilities|Text|ToText(String) (.SS:MS (Utilities|ConvertTimeStamp (Variables|Default|GetElapsedTime))))))