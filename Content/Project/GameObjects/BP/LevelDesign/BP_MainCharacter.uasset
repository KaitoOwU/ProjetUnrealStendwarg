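; Player character that wires together wallrunning, jumping, grappling and two-color switchable glasses, with per-level pickaxe and glasses equipment.
; Trigger volumes feed the wall-move component and its events drive camera lean, while overlaps toggle nearby grapple hooks.
; Controller events swap glasses through timelines animating rotation and dynamic materials, recolored by the game instance.
; KillPlayer stops movement sounds and shows the lose screen with elapsed time.
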(event OnComponentBeginOverlap(GroundCheck)
  (params (OverlappedComponent :type Primitive%20Component%20Object%20Reference) (OtherActor :type Actor%20Object%20Reference) (OtherComp :type Primitive%20Component%20Object%20Reference) (OtherBodyIndex :type Integer) (bFromSweep :type Boolean) (SweepResult :type Hit%20Result%20Structure%20%28by%20ref%29))
  ;[1 1 1] Groundcheck
  (Default|JumpUpdate (Variables|Default|GetBP_WallMoves)))

(event OnComponentEndOverlap(GroundCheck)
  (params (OverlappedComponent :type Primitive%20Component%20Object%20Reference) (OtherActor :type Actor%20Object%20Reference) (OtherComp :type Primitive%20Component%20Object%20Reference) (OtherBodyIndex :type Integer))
  ;[1 1 1] Groundcheck
  (Default|JumpUpdate (Variables|Default|GetBP_WallMoves)))

(event OnComponentBeginOverlap(WallCheckL)
  (params (OverlappedComponent :type Primitive%20Component%20Object%20Reference) (OtherActor :type Actor%20Object%20Reference) (OtherComp :type Primitive%20Component%20Object%20Reference) (OtherBodyIndex :type Integer) (bFromSweep :type Boolean) (SweepResult :type Hit%20Result%20Structure%20%28by%20ref%29))
  ;[1 1 1] WallCheck ON
  (bind _isrunnable (CallFunction|IsWallrunnable OtherActor))
  (if _isrunnable
    (Default|LWRON (Variables|Default|GetBP_WallMoves))))

(event OnComponentEndOverlap(WallCheckR)
  (params (OverlappedComponent :type Primitive%20Component%20Object%20Reference) (OtherActor :type Actor%20Object%20Reference) (OtherComp :type Primitive%20Component%20Object%20Reference) (OtherBodyIndex :type Integer))
  ;[1 1 1] WallCheck OFF
  (bind _isrunnable (CallFunction|IsWallrunnable OtherActor))
  (if _isrunnable
    (Default|RWROFF (Variables|Default|GetBP_WallMoves))))

(event OnComponentBeginOverlap(WallCheckR)
  (params (OverlappedComponent :type Primitive%20Component%20Object%20Reference) (OtherActor :type Actor%20Object%20Reference) (OtherComp :type Primitive%20Component%20Object%20Reference) (OtherBodyIndex :type Integer) (bFromSweep :type Boolean) (SweepResult :type Hit%20Result%20Structure%20%28by%20ref%29))
  ;[1 1 1] WallCheck ON
  (bind _isrunnable (CallFunction|IsWallrunnable OtherActor))
  (if _isrunnable
    (Default|RWRON (Variables|Default|GetBP_WallMoves))))

(event OnComponentEndOverlap(WallCheckL)
  (params (OverlappedComponent :type Primitive%20Component%20Object%20Reference) (OtherActor :type Actor%20Object%20Reference) (OtherComp :type Primitive%20Component%20Object%20Reference) (OtherBodyIndex :type Integer))
  ;[1 1 1] WallCheck OFF
  (bind _isrunnable (CallFunction|IsWallrunnable OtherActor))
  (if _isrunnable
    (Default|LWROFF (Variables|Default|GetBP_WallMoves))))

(event Custom|PickepUpPickaxe
  (bind _mesh (Variables|Character|GetMesh))
  ;[1 1 1] Equip either the pickaxe or the glasses
  (Components|Activation|Activate _mesh false)
  (Rendering|SetVisibility _mesh true true)
  (Variables|/Game/Project/GameObjects/BP/BP_Jumps.BP_Jumps_C|SetIsPickaxeEquipped (Variables|Default|GetBP_Jumps) true))

(event Custom|EDCalled2
  (params (IsWRing :type Boolean) (WasWRRight :type Boolean) (IsLaunching :type Boolean))
  ;[0 1 0.2146] Wallrunning Stance update
  (CallFunction|UpdateWRingStance IsWRing WasWRRight))

(event Custom|EDCalled
  (params (IsWRing :type Boolean) (IsWRingRight :type Boolean))
  ;[0 1 0.2146] Wallrunning Stance update
  (CallFunction|UpdateWRingStance IsWRing IsWRingRight))

(event Custom|ChangeGlasses
  (params (PlaySound :type Boolean))
  (bind _as_pc_main_character (Variables|Default|GetAs%20PC%20Main%20Character))
  (bind _color1material (Variables|Default|GetColor1Material))
  (bind _color2material (Variables|Default|GetColor2Material))
  (bind _currentcolorvar (Variables|/Game/Project/GameObjects/Game/PC_MainCharacter.PC_MainCharacter_C|GetCurrentColorVar _as_pc_main_character))
  ;[1 0.5031 0.7828] Glasses SwitchAnim
  ;;[1 1 1] Change Filter if not already right color
  (if (Utilities|Enum|NotEqual(Enum) _currentcolorvar (Variables|Default|GetCurrentColor))
    (Utilities|FlowControl|Sequence
      (:then_0
        (switch Utilities|FlowControl|Switch|SwitchonE_Colors _currentcolorvar
          (:NewEnumerator0
            ;;[1 1 1] Anim
            (bind _newrotation (Timeline|GlassesAnimRotation PlayFromStart)
              (:Update
                (Transformation|SetRelativeRotation (Variables|Default|Getglasses) (Math|Rotator|MakeRotator 0.0 _newrotation -2.7e+02) false false))
              (:Finished
                (Variables|Default|SetCurrentColor _currentcolorvar))))
          (:NewEnumerator1
            (Timeline|GlassesAnimRotation ReverseFromEnd))))
      (:then_1
        ;;[1 1 1] FadeOut
        (switch Utilities|FlowControl|Switch|SwitchonE_Colors _currentcolorvar
          (:NewEnumerator0
            (bind (_direction _opacity _newior _normals) (Timeline|GlassesAnimOpacity ReverseFromEnd)
              (:Update
                (Rendering|Material|SetScalarParameterValue _color1material "Opacity" _opacity :!class /Script/Engine.MaterialInstanceDynamic)
                (Rendering|Material|SetScalarParameterValue _color1material "IOR" _newior :!class /Script/Engine.MaterialInstanceDynamic)
                (Rendering|Material|SetScalarParameterValue _color1material "NormalsPower" _normals :!class /Script/Engine.MaterialInstanceDynamic)
                (Rendering|Material|SetScalarParameterValue _color1material "GlassEffect" _normals :!class /Script/Engine.MaterialInstanceDynamic)
                (bind (_direction_2 _opacity_2 _newior_2 _normals_2) (Timeline|Timeline_1 PlayFromStart)
                  (:Update
                    (Rendering|Material|SetScalarParameterValue _color2material "Opacity" _opacity_2 :!class /Script/Engine.MaterialInstanceDynamic)
                    (Rendering|Material|SetScalarParameterValue _color2material "IOR" _newior_2 :!class /Script/Engine.MaterialInstanceDynamic)
                    (Rendering|Material|SetScalarParameterValue _color2material "NormalsPower" _normals_2 :!class /Script/Engine.MaterialInstanceDynamic)
                    (Rendering|Material|SetScalarParameterValue _color2material "GlassEffect" _normals_2 :!class /Script/Engine.MaterialInstanceDynamic))))))
          (:NewEnumerator1
            (bind (_direction_3 _opacity_3 _newior_3 _normals_3) (Timeline|Timeline ReverseFromEnd)
              (:Update
                (Rendering|Material|SetScalarParameterValue _color2material "Opacity" _opacity_3 :!class /Script/Engine.MaterialInstanceDynamic)
                (Rendering|Material|SetScalarParameterValue _color2material "IOR" _newior_3 :!class /Script/Engine.MaterialInstanceDynamic)
                (Rendering|Material|SetScalarParameterValue _color2material "NormalsPower" _normals_3 :!class /Script/Engine.MaterialInstanceDynamic)
                (Rendering|Material|SetScalarParameterValue _color2material "GlassEffect" _normals_3 :!class /Script/Engine.MaterialInstanceDynamic)
                (bind (_direction_4 _opacity_4 _newior_4 _normals_4) (Timeline|Timeline_3 PlayFromStart)
                  (:Update
                    (Rendering|Material|SetScalarParameterValue _color1material "Opacity" _opacity_4 :!class /Script/Engine.MaterialInstanceDynamic)
                    (Rendering|Material|SetScalarParameterValue _color1material "IOR" _newior_4 :!class /Script/Engine.MaterialInstanceDynamic)
                    (Rendering|Material|SetScalarParameterValue _color1material "NormalsPower" _normals_4 :!class /Script/Engine.MaterialInstanceDynamic)
                    (Rendering|Material|SetScalarParameterValue _color1material "GlassEffect" _normals_4 :!class /Script/Engine.MaterialInstanceDynamic)))))))))))

(event Custom|PickedUpGlasses
  (bind _glasses (Variables|Default|Getglasses))
  ;[1 1 1] Equip either the pickaxe or the glasses
  (Components|Activation|Activate _glasses false)
  (Rendering|SetVisibility _glasses true true)
  (Variables|/Game/Project/GameObjects/Game/PC_MainCharacter.PC_MainCharacter_C|SetAreGlassesEquipped (Variables|Default|GetAs%20PC%20Main%20Character) true))

(event Custom|CustomGlassesColor
  (params (ColorValue :type Float%20%28double-precision%29) (AffectedColorBlock :type E_Colors%20Enum :default "NewEnumerator0"))
  ;[1 0.2219 0.4924] Custom Colors
  (CallFunction|ChangeGlassesColor ColorValue AffectedColorBlock))

(event EventBeginPlay
  (bind _returnvalue (Game|GetPlayerCharacter 0))
  (bind _bp_wallmoves (Variables|Default|GetBP_WallMoves))
  (bind _charactermovement (Variables|/Script/Engine.Character|GetCharacterMovement _returnvalue))
  (Components|Sphere|SetSphereRadius (Variables|Default|GetHookCollider) (Variables|/Game/Project/GameObjects/BP/BP_GrapplingHook.BP_GrapplingHook_C|GetGrapplingHookRange (Variables|Default|GetBP_GrapplingHook)) true)
  (bind _aspc_main_character (Utilities|Casting|CastToPC_MainCharacter (Game|GetPlayerController 0)))
  (Variables|Default|SetAs%20PC%20Main%20Character _aspc_main_character)
  ;[1 1 1] Sets Character Values
  (Variables|/Script/Engine.CharacterMovementComponent|SetGravityScale _charactermovement (Variables|Default|GetGravityScaleSet))
  (Variables|/Script/Engine.CharacterMovementComponent|SetMaxWalkSpeed _charactermovement (Variables|Default|GetCharacterSpeed))
  (Variables|/Script/Engine.CharacterMovementComponent|SetAirControl _charactermovement (Variables|Default|GetAirControlSet))
  ;[0 1 0.2146] Wallrunning Stance update
  (EventDispatchers|BindEventtoEDWallrunningON _bp_wallmoves (delegate Custom|EDCalled))
  (EventDispatchers|BindEventtoEDWallrunningOFF _bp_wallmoves (delegate Custom|EDCalled2))
  ;[1 0.5031 0.7828] Glasses SwitchAnim
  (EventDispatchers|BindEventtoEDChangeGlasses (Variables|Default|GetAs%20PC%20Main%20Character) (delegate Custom|ChangeGlasses))
  (CallFunction|GetGlassesMaterials)
  (Default|CallEDChangeGlasses (Variables|Default|GetAs%20PC%20Main%20Character) false)
  ;[1 0.2219 0.4924] Custom Colors
  (bind _asgi_stendvarg (Utilities|Casting|CastToGI_Stendvarg (Game|GetGameInstance)))
  (bind _output_get (Variables|Default|SetGameInstance _asgi_stendvarg))
  (EventDispatchers|BindEventtoUpdateBlockColors _output_get (delegate Custom|CustomGlassesColor))
  (CallFunction|CheckEquippable)
  (Components|Activation|SetActive (Variables|Default|GetSparks) false false))

(event Collision|EventActorBeginOverlap
  (params (OtherActor :type Actor%20Object%20Reference))
  ;[1 1 1] Makes the hooks grappleable when near them
  (if (Utilities|DoesObjectImplementInterface OtherActor "/Game/Project/GameObjects/BP/I_IsHook.I_IsHook_C")
    (bind _asbp_hook (Utilities|Casting|CastToBP_Hook OtherActor))
    (Default|SetActive _asbp_hook true)))

(event Collision|EventActorEndOverlap
  (params (OtherActor :type Actor%20Object%20Reference))
  ;[1 1 1] Makes the hooks grappleable when near them
  (if (Utilities|DoesObjectImplementInterface OtherActor "/Game/Project/GameObjects/BP/I_IsHook.I_IsHook_C")
    (bind _asbp_hook (Utilities|Casting|CastToBP_Hook OtherActor))
    (Default|SetActive _asbp_hook false)))

(fn ConstructionScript)

(fn IsWallrunnable
  (params (InputActor :type Actor%20Object%20Reference))
  (bind _returnvalue (Actor|GetComponentbyClass InputActor "/Game/Project/GameObjects/BP/BP_WallRunableComponnent.BP_WallRunableComponnent_C"))
  (Utilities|IsValid _returnvalue
    (:Is%20Valid
      (return InputActor (Variables|/Game/Project/GameObjects/BP/BP_WallRunableComponnent.BP_WallRunableComponnent_C|GetIsRunnable _returnvalue)))
    (:Is%20Not%20Valid
      (Development|PrintString "Isn't a wall" true true "(R=1.000000,G=0.084190,B=0.000000,A=1.000000)" 1.0))))

(fn UpdateWRingStance
  (params (IsWRing :type Boolean) (Right :type Boolean))
  (bind _as_pc_main_character (Variables|Default|GetAs%20PC%20Main%20Character))
  (bind _as_pc_main_character_2 (Variables|Default|GetAs%20PC%20Main%20Character))
  (bind _cameralean (Variables|Default|GetCameraLean))
  (bind _returnvalue (* _cameralean -1.0))
  (if IsWRing
    (if Right
      (Class|PlayerController|AddRollInput _as_pc_main_character_2 _returnvalue)
      (else
        (Class|PlayerController|AddRollInput _as_pc_main_character_2 _cameralean)))
    (elif Right
      (Class|PlayerController|AddRollInput _as_pc_main_character _cameralean)
      (else
        (Class|PlayerController|AddRollInput _as_pc_main_character _returnvalue)))))

(fn KillPlayer
  (bind _returnvalue (Game|GetPlayerController 0))
  (bind _slidesound (Variables|/Game/Project/GameObjects/Game/PC_MainCharacter.PC_MainCharacter_C|GetSlideSound (Variables|Default|GetAs%20PC%20Main%20Character))
    (:then
      (Audio|Components|Audio|Stop _slidesound))
    (:else
      _))
  (bind _wallrunsound (Variables|/Game/Project/GameObjects/BP/BP_WallMoves.BP_WallMoves_C|GetWallRunSound (Variables|Default|GetBP_WallMoves))
    (:then
      (Audio|Components|Audio|Stop _wallrunsound))
    (:else
      _))
  (Variables|Default|SetIsDead true)
  (Viewport|RemoveAllWidgets)
  (bind _returnvalue_2 (UserInterface|CreateWidget "/Game/Project/UMG/UW_LoseScreen.UW_LoseScreen_C" (Variables|Default|GetAs%20PC%20Main%20Character)))
  (bind _returnvalue_3 (Actor|GetActorOfClass "/Game/Project/GameObjects/BP/LevelDesign/BP_UIManager.BP_UIManager_C"))
  (bind _elapsed_time (Default|GetConvertedElapsedTime _returnvalue_3))
  (Variables|/Script/UMG.TextBlock|SetText (Variables|/Game/Project/UMG/UW_LoseScreen.UW_LoseScreen_C|GetTime _returnvalue_2) _elapsed_time)
  (UserInterface|Viewport|AddtoViewport _returnvalue_2 0)
  (Input|SetInputModeUIOnly _returnvalue 0 "DoNotLock" true)
  (Variables|/Script/Engine.PlayerController|SetbShowMouseCursor _returnvalue true))

(fn GetGlassesMaterials
  (bind _glasses (Variables|Default|Getglasses))
  (bind _returnvalue (Rendering|Material|CreateDynamicMaterialInstance _glasses 2 "/Game/Project/Materials/Glasses/MI_GlassesColor1.MI_GlassesColor1" "Material1" :!class /Script/Engine.PrimitiveComponent))
  (Utilities|IsValid _returnvalue
    (:Is%20Valid
      (Variables|Default|SetColor1Material _returnvalue)
      (bind _returnvalue_2 (Rendering|Material|CreateDynamicMaterialInstance _glasses 3 "/Game/Project/Materials/Glasses/MI_GlassesColor2.MI_GlassesColor2" "Material2" :!class /Script/Engine.PrimitiveComponent))
      (Utilities|IsValid _returnvalue_2
        (:Is%20Valid
          (Variables|Default|SetColor2Material _returnvalue_2))))))

(fn ChangeGlassesColor
  (params (NewColor :type Float%20%28double-precision%29) (AffectedColor :type E_Colors%20Enum :default "NewEnumerator0"))
  (bind _returnvalue (Class|KismetMathLibrary|HSVtoRGB NewColor 1.0 1.0 1.0))
  (switch Utilities|FlowControl|Switch|SwitchonE_Colors AffectedColor
    (:NewEnumerator0
      (Rendering|Material|SetVectorParameterValue (Variables|Default|GetColor1Material) "BaseColor" _returnvalue :!class /Script/Engine.MaterialInstanceDynamic))
    (:NewEnumerator1
      (Rendering|Material|SetVectorParameterValue (Variables|Default|GetColor2Material) "BaseColor" _returnvalue :!class /Script/Engine.MaterialInstanceDynamic))))

(fn AnimateChain
  (params (End :type Vector) (IsMissed :type Boolean)))

(fn CheckEquippable
  ;[1 1 1] Checks if the pickaxe or the glasses should be removed from the player
  (bind _asgi_stendvarg (Utilities|Casting|CastToGI_Stendvarg (Game|GetGameInstance)))
  (Utilities|FlowControl|Sequence
    (:then_0
      (if (not (.PickaxeActive (Utilities|Struct|BreakS_LevelData (Variables|/Game/Project/GameObjects/Game/GI_Stendvarg.GI_Stendvarg_C|GetCurrentLevelData _asgi_stendvarg))))
        (Components|Activation|Deactivate (Variables|Character|GetMesh))
        (Rendering|SetVisibility (Variables|Character|GetMesh) false true)))
    (:then_1
      (if (not (.GlassesActive (Utilities|Struct|BreakS_LevelData (Variables|/Game/Project/GameObjects/Game/GI_Stendvarg.GI_Stendvarg_C|GetCurrentLevelData _asgi_stendvarg))))
        (Components|Activation|Deactivate (Variables|Default|Getglasses))
        (Rendering|SetVisibility (Variables|Default|Getglasses) false true)))))