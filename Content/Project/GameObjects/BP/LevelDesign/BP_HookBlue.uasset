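; BP_HookBlue is a level-design hook point for the main character's grappling hook.
; On BeginPlay it sizes its activation collider to the character's grappling hook range, while the construction script sizes a second collider from SphereSize.
; A separate trigger zone switches the point light on and off as the main character enters and leaves.
; SetActive swaps the sphere between on and off materials to show hook state.
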(event OnComponentBeginOverlap(DansTriggerZone)
  (params (OverlappedComponent :type Primitive%20Component%20Object%20Reference) (OtherActor :type Actor%20Object%20Reference) (OtherComp :type Primitive%20Component%20Object%20Reference) (OtherBodyIndex :type Integer) (bFromSweep :type Boolean) (SweepResult :type Hit%20Result%20Structure%20%28by%20ref%29))
  (Utilities|Casting|CastToBP_MainCharacter OtherActor)
  (Rendering|Components|Light|SetIntensity (Variables|Default|GetPointLight) 1e+04))

(event OnComponentEndOverlap(DansTriggerZone)
  (params (OverlappedComponent :type Primitive%20Component%20Object%20Reference) (OtherActor :type Actor%20Object%20Reference) (OtherComp :type Primitive%20Component%20Object%20Reference) (OtherBodyIndex :type Integer))
  (Utilities|Casting|CastToBP_MainCharacter OtherActor)
  (Rendering|Components|Light|SetIntensity (Variables|Default|GetPointLight) 0.0))

(event EventBeginPlay
  (bind _returnvalue (Actor|GetActorOfClass "/Game/Project/GameObjects/BP/LevelDesign/BP_MainCharacter.BP_MainCharacter_C"))
  (Components|Sphere|SetSphereRadius (Variables|Default|GetHookActivationByPlayerCollider) (Variables|/Game/Project/GameObjects/BP/BP_GrapplingHook.BP_GrapplingHook_C|GetGrapplingHookRange (Variables|/Game/Project/GameObjects/BP/LevelDesign/BP_MainCharacter.BP_MainCharacter_C|GetBP_GrapplingHook _returnvalue)) true))

(fn ConstructionScript
  (Components|Sphere|SetSphereRadius (Variables|Default|GetSphereSizeCollider) (Variables|Default|GetSphereSize) true))

(fn SetActive
  (params (Active :type Boolean))
  (bind _sphere (Variables|Default|GetSphere))
  (if Active
    (Rendering|Material|SetMaterial _sphere 0 "/Game/Project/Materials/M_GrapplingHookOn.M_GrapplingHookOn")
    (else
      (Rendering|Material|SetMaterial _sphere 0 "/Game/Project/Materials/M_GrapplingHookOff.M_GrapplingHookOff"))))