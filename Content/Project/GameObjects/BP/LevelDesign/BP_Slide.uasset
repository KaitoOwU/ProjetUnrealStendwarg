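; BP_Slide is a level-design slide Blueprint that pushes the main character along a given direction.
; BeginPlay caches the BP_MainCharacter, and Tick advances a timer while IsSliding until SlideDuration ends.
; Impulse resets the timer and sets the character's location once, so its lerp always yields the full offset, an instant jump.
; Nothing here sets IsSliding true or moves the character on Tick, and a debug print remains.
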(event EventBeginPlay
  (bind _returnvalue (Actor|GetActorOfClass "/Game/Project/GameObjects/BP/LevelDesign/BP_MainCharacter.BP_MainCharacter_C"))
  (Variables|Default|SetMainCharacter _returnvalue))

(event EventTick
  (params (DeltaSeconds :type Float%20%28single-precision%29))
  (if (Variables|Default|GetIsSliding)
    (bind _output_get (Variables|Default|SetTimer (+ DeltaSeconds (Variables|Default|GetTimer))))
    (Variables|Default|SetIsSliding (< _output_get (Variables|Default|GetSlideDuration)))))

(fn Impulse
  (params (Direction :type Vector))
  (bind _maincharacter (Variables|Default|GetMainCharacter))
  (bind _returnvalue (Transformation|GetActorLocation _maincharacter))
  (Variables|Default|SetTimer 0.0)
  (Transformation|SetActorLocation _maincharacter (Math|Vector|Lerp(Vector) (+ (* Direction 1e+02) _returnvalue) _returnvalue (/ (Variables|Default|GetTimer) (Variables|Default|GetSlideDuration))) false false)
  (Development|PrintString "Hello" true true "(R=0.000000,G=0.660000,B=1.000000,A=1.000000)" (/ (Variables|Default|GetTimer) (Variables|Default|GetSlideDuration))))