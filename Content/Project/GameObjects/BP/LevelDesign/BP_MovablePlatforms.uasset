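; Level-design Blueprint for a movable platform that travels between a start and an end point.
; The construction script places the StartPosition and EndPosition components at stored world-space vectors.
; On BeginPlay it records both components' world locations, then destroys the EndPosition component.
; The MovePlatforms timeline then lerps StartPosition between the recorded locations, without sweep.
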(event EventBeginPlay
  (Variables|Default|SetStartPositionVector (Transformation|GetWorldLocation (Variables|Default|GetStartPosition)))
  (Variables|Default|SetEndPositionVector (Transformation|GetWorldLocation (Variables|Default|GetEndPosition)))
  (Components|DestroyComponent (Variables|Default|GetEndPosition))
  (bind _value (Timeline|Move%20Platforms Play)
    (:Update
      (Transformation|SetWorldLocation (Variables|Default|GetStartPosition) (Math|Vector|Lerp(Vector) (Variables|Default|GetStartPositionVector) (Variables|Default|GetEndPositionVector) _value) false false))))

(fn ConstructionScript
  (Transformation|SetWorldLocation (Variables|Default|GetStartPosition) (Variables|Default|GetStartPositionVector) false false)
  (Transformation|SetWorldLocation (Variables|Default|GetEndPosition) (Variables|Default|GetEndPositionVector) false false))