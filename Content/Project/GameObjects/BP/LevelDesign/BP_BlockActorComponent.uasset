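; Actor component for color-filtered level blocks that shows or hides its owner's static mesh as the player changes glasses.
; On BeginPlay it caches the mesh and binds to the glasses-change event on PC_MainCharacter.
; Each change hides the block when its color matches the active filter and shows it when they differ.
; The switch then sets collision to PhysicsOnly in either case, leaving a NoCollision call unused.
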(event Custom|SwitchBlockVisibility
  (CallFunction|SwitchVisibility (stale EventBeginPlay _aspc_main_character)))

(event EventBeginPlay
  (Variables|Default|SetBlockMesh (Actor|GetComponentbyClass (Components|GetOwner self) "/Script/Engine.StaticMeshComponent"))
  (bind _aspc_main_character (Utilities|Casting|CastToPC_MainCharacter (Game|GetPlayerController 0)))
  (EventDispatchers|BindEventtoEDChangeGlasses _aspc_main_character (delegate Custom|SwitchBlockVisibility)))

(fn SwitchVisibility
  (params (playerController :type PC%20Main%20Character%20Object%20Reference))
  (bind _blockmesh (Variables|Default|GetBlockMesh))
  (bind _blockcolor (Variables|Default|GetBlockColor))
  ;[1 1 1] Switch Visibility based on current active filter, and block color
  (switch Utilities|FlowControl|Switch|SwitchonE_Colors (Variables|/Game/Project/GameObjects/Game/PC_MainCharacter.PC_MainCharacter_C|GetCurrentColorVar playerController)
    (:NewEnumerator0
      (switch Utilities|FlowControl|Switch|SwitchonE_Colors _blockcolor
        (:NewEnumerator0
          (Rendering|SetVisibility _blockmesh false false :!label _label))
        (:NewEnumerator1
          (Rendering|SetVisibility _blockmesh true false :!label _label_2))))
    (:NewEnumerator1
      (switch Utilities|FlowControl|Switch|SwitchonE_Colors _blockcolor
        (:NewEnumerator0
          (goto _label_2))
        (:NewEnumerator1
          (goto _label)))))
  (Collision|SetCollisionEnabled _blockmesh "PhysicsOnly"))